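; TreasureItem_Blueprint is a collectible treasure pickup that plays a sound while a character is nearby.
; When a Character overlaps the Item component, it increments the TreasureItems count on ThirdPersonGameMode and destroys itself.
; A separate Sound_Collision volume plays TreasureNoise while a Character is inside and stops it on exit, with the sound silenced at BeginPlay.
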(event OnComponentBeginOverlap(Item)
  (params (OverlappedComponent :type Primitive%20Component%20Object%20Reference) (OtherActor :type Actor%20Object%20Reference) (OtherComp :type Primitive%20Component%20Object%20Reference) (OtherBodyIndex :type Integer) (bFromSweep :type Boolean) (SweepResult :type Hit%20Result%20Structure%20%28by%20ref%29))
  (Utilities|Casting|CastToCharacter OtherActor)
  (bind _asthird_person_game_mode (Utilities|Casting|CastToThirdPersonGameMode (Game|GetGameMode)))
  (Variables|/Game/ThirdPersonBP/Blueprints/ThirdPersonGameMode.ThirdPersonGameMode_C|SetTreasureItems _asthird_person_game_mode (+ (Variables|/Game/ThirdPersonBP/Blueprints/ThirdPersonGameMode.ThirdPersonGameMode_C|GetTreasureItems _asthird_person_game_mode) 1))
  (Actor|DestroyActor))

(event OnComponentBeginOverlap(Sound_Collision)
  (params (OverlappedComponent :type Primitive%20Component%20Object%20Reference) (OtherActor :type Actor%20Object%20Reference) (OtherComp :type Primitive%20Component%20Object%20Reference) (OtherBodyIndex :type Integer) (bFromSweep :type Boolean) (SweepResult :type Hit%20Result%20Structure%20%28by%20ref%29))
  (Utilities|Casting|CastToCharacter OtherActor)
  (Audio|Components|Audio|Play (Variables|Default|GetTreasure_Noise) 0.0))

(event OnComponentEndOverlap(Sound_Collision)
  (params (OverlappedComponent :type Primitive%20Component%20Object%20Reference) (OtherActor :type Actor%20Object%20Reference) (OtherComp :type Primitive%20Component%20Object%20Reference) (OtherBodyIndex :type Integer))
  (Utilities|Casting|CastToCharacter OtherActor)
  (Audio|Components|Audio|Stop (Variables|Default|GetTreasure_Noise)))

(event EventBeginPlay
  (Audio|Components|Audio|Stop (Variables|Default|GetTreasure_Noise)))

(fn ConstructionScript)